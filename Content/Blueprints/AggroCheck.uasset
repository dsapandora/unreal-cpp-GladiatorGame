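; AggroCheck is a Behavior Tree tick node that detects targets around the AI's controlled pawn.
; Each tick, a debug-drawn multi-sphere trace gathers nearby objects of the desired types, then a Camera-channel line trace checks line of sight to each.
; Visible hits write TargetToFollow and TargetLocation to the Blackboard; blocked hits clear only TargetToFollow, so the last hit processed decides the target.
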(event `self.ReceiveTick`
  (params (OwnerActor :type "Actor Object Reference") (DeltaSeconds :type "Float (single-precision)"))
  (bind _asaiblueprint_bt_c (cast `/Game/Blueprints/AIBlueprint_BT` OwnerActor))
  (set `self.AIBlueprint_CONT REF` _asaiblueprint_bt_c)
  (bind _returnvalue (`Actor.K2_GetActorLocation` (`Controller.GetControlledPawn` _asaiblueprint_bt_c)))
  (set `self.MyLocation` _returnvalue)
  (bind _outhits (`KismetSystemLibrary.SphereTraceMultiForObjects` _returnvalue (+ _returnvalue (0.0 0.0 5.0)) 1000.0 (`self.DesiredObjectTypes`) false (`|MakeArray` (`Controller.GetControlledPawn` (`self.AIBlueprint_CONT REF`)) :!type "Actor Object Reference") "ForDuration"))
  (for _array_element _outhits
    (bind (_location _normal _impactpoint _impactnormal _physmat _hitactor) (`GameplayStatics.BreakHitResult` _array_element))
    (bind _outhit (`KismetSystemLibrary.LineTraceSingle` (`self.MyLocation`) (`Actor.K2_GetActorLocation` _hitactor) "TraceTypeQuery2" false (`|MakeArray` (`Controller.GetControlledPawn` (`self.AIBlueprint_CONT REF`)) :!type "Actor Object Reference") "ForDuration"))
    (bind (_location_2 _normal_2 _impactpoint_2 _impactnormal_2 _physmat_2 _hitactor_2) (`GameplayStatics.BreakHitResult` _outhit))
    (if (== _hitactor _hitactor_2)
      (`BTFunctionLibrary.SetBlackboardValueAsObject` (`self.TargetToFollow`) _hitactor_2)
      (`BTFunctionLibrary.SetBlackboardValueAsVector` (`self.TargetLocation`) (`Actor.K2_GetActorLocation` _hitactor_2))
      (else
        (`BTFunctionLibrary.SetBlackboardValueAsObject` (`self.TargetToFollow`))))))