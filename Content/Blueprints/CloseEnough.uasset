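; CloseEnough is a Behavior Tree decorator that checks the AI pawn's distance to the actor in the TargetToFollow blackboard value.
; It casts the owner to AIBlueprint_BT and compares the pawn-to-target distance against AcceptableDistance.
; Despite its name, it passes when the target is at or beyond that distance and fails when closer.
; A failed cast leaves the check unfinished.
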(event `self.ReceiveConditionCheck`
  (params (OwnerActor :type "Actor Object Reference"))
  (bind _asaiblueprint_bt_c (cast `/Game/Blueprints/AIBlueprint_BT` OwnerActor))
  (set `self.AIBlueprint_CONT REF` _asaiblueprint_bt_c)
  (if (>= (`KismetMathLibrary.VSize` (- (`Actor.K2_GetActorLocation` (`BTFunctionLibrary.GetBlackboardValueAsActor` (`self.TargetToFollow`))) (`Actor.K2_GetActorLocation` (`Controller.GetControlledPawn` (`self.AIBlueprint_CONT REF`))))) (`self.AcceptableDistance`))
    (`self.FinishConditionCheck` true)
    (else
      (`self.FinishConditionCheck` false))))