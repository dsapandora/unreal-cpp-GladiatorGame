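; Behavior tree task RapidMoveTo that keeps an enemy gladiator moving to a spot near its blackboard TargetToFollow actor.
; On execute it caches the AI controller and opens a gate, so every Tick reissues AIMoveTo with a fresh destination.
; The destination is the target's location offset along the gladiator's normalized MoveDir by AcceptableDistance.
; A successful move finishes the task and closes the gate; failed moves do not finish it.
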(event `self.ReceiveTick`
  (params (OwnerActor :type "Actor Object Reference") (DeltaSeconds :type "Float (single-precision)"))
  (`/Engine/EditorBlueprintResources/StandardMacros.Gate` true :!label _label
    (:`Exit`
      (bind _asaenemygladiatorblueprint_c (cast `/Game/Blueprints/AEnemyGladiatorBlueprint` (`Controller.GetControlledPawn` (`self.AIBlueprint_CONT REF`))))
      (`|AIMoveTo` (`Controller.GetControlledPawn` (`self.AIBlueprint_CONT REF`)) (+ (* (`KismetMathLibrary.Normal` (`AGladiatorCode.moveDir` _asaenemygladiatorblueprint_c)) (`self.AcceptableDistance`)) (`Actor.K2_GetActorLocation` (`BTFunctionLibrary.GetBlackboardValueAsActor` (`self.TargetToFollow`)))) null 50.0
        (:`OnSuccess`
          (`self.FinishExecute` true)
          (`self.CloseGate`))))))

(event `self.ReceiveExecute`
  (params (OwnerActor :type "Actor Object Reference"))
  (bind _asaiblueprint_bt_c (cast `/Game/Blueprints/AIBlueprint_BT` OwnerActor))
  (set `self.AIBlueprint_CONT REF` _asaiblueprint_bt_c)
  (goto _label :!via `Open`))

(event `CloseGate`
  (goto _label :!via `Close`))