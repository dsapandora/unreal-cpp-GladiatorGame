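; Player-controlled gladiator character with movement, mouse look, a timed attack state and a death state.
; Move inputs follow control yaw and are ignored while attacking, while mouse input turns the controller, with pitch scaled down.
; Attack sets IsAttack, then clears it after a fixed delay just under a second.
; Tick sets IsDead whenever Life exactly equals zero and clears it otherwise.
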(event `InputAxis|MoveForward`
  (params (AxisValue :type "Float (single-precision)"))
  ;[1 1 1] Input Mouvement
  (if (not (`self.IsAttack?`))
    (`self.AddMovementInput` (`KismetMathLibrary.GetForwardVector` (`KismetMathLibrary.MakeRot` 0.0 (.yaw (`self.GetControlRotation`)))) AxisValue)))

(event `InputAxis|MoveRight`
  (params (AxisValue :type "Float (single-precision)"))
  ;[1 1 1] Input Mouvement
  (if (not (`self.IsAttack?`))
    (`self.AddMovementInput` (`KismetMathLibrary.GetRightVector` (`KismetMathLibrary.MakeRot` 0.0 (.yaw (`self.GetControlRotation`)))) AxisValue)))

(event `InputAxis|Turn`
  (params (AxisValue :type "Float (single-precision)"))
  ;[1 1 1] Mouse rotation
  (`self.AddControllerYawInput` AxisValue))

(event `InputAction|Attack`
  ;[1 1 1] Attack State
  (:`Pressed`
    (set `self.IsAttack?` true)
    (`KismetSystemLibrary.Delay` 0.833)
    (set `self.IsAttack?` false)))

(event `InputAxis|LookUp`
  (params (AxisValue :type "Float (single-precision)"))
  ;[1 1 1] Mouse rotation
  (`self.AddControllerPitchInput` (* AxisValue 0.3)))

(event `self.ReceiveTick`
  (params (DeltaSeconds :type "Float (single-precision)"))
  ;[1 1 1] Death State
  (if (== (`self.life`) 0)
    (set `self.IsDead?` true)
    (else
      (set `self.IsDead?` false))))

(fn `UserConstructionScript`)