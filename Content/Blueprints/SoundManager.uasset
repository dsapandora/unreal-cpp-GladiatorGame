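; SoundManager drives adaptive arena music that escalates with kills and ends with a win or lose sting.
; On BeginPlay it starts five music stems together as attached audio components, muting all but the first.
; Events kill1 to kill4 each crossfade from the current stem to the next over one second.
; The endofmatch event fades out every stem and plays the result cue based on the Victory flag.
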(event `self.ReceiveBeginPlay`
  (bind _audiocomponents (`self.AudioComponents`))
  (bind _defaultsceneroot (`self.DefaultSceneRoot`))
  ;[1 1 1] Sound Init
  (`|ExecutionSequence`
    (:`then_0`
      (bind _returnvalue (`GameplayStatics.PlaySoundAttached` "/Game/Audio/Cue/MUS/MUS_arena_stem01.MUS_arena_stem01" _defaultsceneroot "None" (0.0 0.0 0.0) "EAttachLocation::KeepRelativeOffset" false 1.0))
      (`KismetArrayLibrary.Array_Set` _audiocomponents 0 _returnvalue))
    (:`then_1`
      (bind _returnvalue_2 (`GameplayStatics.PlaySoundAttached` "/Game/Audio/Cue/MUS/MUS_arena_stem02.MUS_arena_stem02" _defaultsceneroot "None" (0.0 0.0 0.0) "EAttachLocation::KeepRelativeOffset" false 1.0))
      (`KismetArrayLibrary.Array_Set` _audiocomponents 1 _returnvalue_2)
      (`AudioComponent.AdjustVolume` (`KismetArrayLibrary.Array_Get` _audiocomponents 1) 0.0 0.0))
    (:`then_2`
      (bind _returnvalue_3 (`GameplayStatics.PlaySoundAttached` "/Game/Audio/Cue/MUS/MUS_arena_stem03.MUS_arena_stem03" _defaultsceneroot "None" (0.0 0.0 0.0) "EAttachLocation::KeepRelativeOffset" false 1.0))
      (`KismetArrayLibrary.Array_Set` _audiocomponents 2 _returnvalue_3)
      (`AudioComponent.AdjustVolume` (`KismetArrayLibrary.Array_Get` _audiocomponents 2) 0.0 0.0))
    (:`then_3`
      (bind _returnvalue_4 (`GameplayStatics.PlaySoundAttached` "/Game/Audio/Cue/MUS/MUS_arena_stem04.MUS_arena_stem04" _defaultsceneroot "None" (0.0 0.0 0.0) "EAttachLocation::KeepRelativeOffset" false 1.0))
      (`KismetArrayLibrary.Array_Set` _audiocomponents 3 _returnvalue_4)
      (`AudioComponent.AdjustVolume` (`KismetArrayLibrary.Array_Get` _audiocomponents 3) 0.0 0.0))
    (:`then_4`
      (bind _returnvalue_5 (`GameplayStatics.PlaySoundAttached` "/Game/Audio/Cue/MUS/MUS_arena_stem05.MUS_arena_stem05" _defaultsceneroot "None" (0.0 0.0 0.0) "EAttachLocation::KeepRelativeOffset" false 1.0))
      (`KismetArrayLibrary.Array_Set` _audiocomponents 4 _returnvalue_5)
      (`AudioComponent.AdjustVolume` (`KismetArrayLibrary.Array_Get` _audiocomponents 4) 0.0 0.0))))

(event `kill1`
  (bind _audiocomponents (`self.AudioComponents`))
  ;[1 1 1] Sound Event
  (`|ExecutionSequence`
    (:`then_0`
      (`AudioComponent.AdjustVolume` (`KismetArrayLibrary.Array_Get` _audiocomponents) 1.0 0.0 :!label _label))
    (:`then_1`
      (`AudioComponent.AdjustVolume` (`KismetArrayLibrary.Array_Get` _audiocomponents 1) 1.0 1.0))))

(event `kill2`
  (bind _audiocomponents (`self.AudioComponents`))
  ;[1 1 1] Sound Event
  (`|ExecutionSequence`
    (:`then_0`
      (`AudioComponent.AdjustVolume` (`KismetArrayLibrary.Array_Get` _audiocomponents 1) 1.0 0.0 :!label _label_2))
    (:`then_1`
      (`AudioComponent.AdjustVolume` (`KismetArrayLibrary.Array_Get` _audiocomponents 2) 1.0 1.0))))

(event `kill3`
  (bind _audiocomponents (`self.AudioComponents`))
  ;[1 1 1] Sound Event
  (`|ExecutionSequence`
    (:`then_0`
      (`AudioComponent.AdjustVolume` (`KismetArrayLibrary.Array_Get` _audiocomponents 2) 1.0 0.0 :!label _label_3))
    (:`then_1`
      (`AudioComponent.AdjustVolume` (`KismetArrayLibrary.Array_Get` _audiocomponents 3) 1.0 1.0))))

(event `kill4`
  (bind _audiocomponents (`self.AudioComponents`))
  ;[1 1 1] Sound Event
  (`|ExecutionSequence`
    (:`then_0`
      (`AudioComponent.AdjustVolume` (`KismetArrayLibrary.Array_Get` _audiocomponents 3) 1.0 0.0 :!label _label_4))
    (:`then_1`
      (`AudioComponent.AdjustVolume` (`KismetArrayLibrary.Array_Get` _audiocomponents 4) 1.0 1.0))))

(event `endofmatch`
  ;[1 1 1] Sound Event
  (`|ExecutionSequence`
    (:`then_0`
      (`AudioComponent.AdjustVolume` (`KismetArrayLibrary.Array_Get` (`self.AudioComponents`) 4) 1.0 0.0))
    (:`then_1`
      (if (`self.Victory`)
        (`GameplayStatics.PlaySoundAtLocation` "/Game/Audio/Cue/MUS/MUS_arena_win.MUS_arena_win")
        (else
          (`GameplayStatics.PlaySoundAtLocation` "/Game/Audio/Cue/MUS/Mus_arena_lose.Mus_arena_lose"))))
    (:`then_2`
      (goto _label))
    (:`then_3`
      (goto _label_2))
    (:`then_4`
      (goto _label_3))
    (:`then_5`
      (goto _label_4))))

(fn `UserConstructionScript`)